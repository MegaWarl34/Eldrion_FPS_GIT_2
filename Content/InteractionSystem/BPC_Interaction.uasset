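; BPC_Interaction is an actor component that finds interactable actors in front of its owner and triggers them on input.
; A looping timer sphere-traces a short distance forward, stores any hit actor implementing BPI_Interaction as the target, and shows or clears its look-at message in the HUD.
; IA_Interaction hands the target to its BPC_ItemData component if present, otherwise calls its interaction interface messages.
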(event Custom|Begin%20Interaction
  (Utilities|Time|SetTimerbyEvent (delegate Custom|UpdateInteraction) 0.2 true))

(event Custom|UpdateInteraction
  (CallFunction|InteractionTrace))

(event Input|EnhancedActionEvents|EnhancedInputActionIA_Interaction
  (params (ActionValue :type Boolean) (ElapsedSeconds :type Float%20%28double-precision%29) (TriggeredSeconds :type Float%20%28double-precision%29) (InputAction :type Input%20Action%20Object%20Reference :default "/Game/ThirdPerson/Input/Actions/IA_Interaction.IA_Interaction"))
  (bind _returnvalue (Components|GetOwner))
  (:Started
    (bind _target_actor (Variables|Default|GetTarget%20actor)
      (:then
        (Utilities|IsValid (Actor|GetComponentbyClass _target_actor "/Game/Inventory_System/ItemData/BPC_ItemData.BPC_ItemData_C")
          (:Is%20Valid
            (Default|Interactwith (Actor|GetComponentbyClass _target_actor "/Game/Inventory_System/ItemData/BPC_ItemData.BPC_ItemData_C") _returnvalue))
          (:Is%20Not%20Valid
            (Class|BPIInteraction|Interactwith(Message) (Variables|Default|GetTarget%20actor) _returnvalue)
            (Class|BPIInteraction|InteractAction(Message) (Variables|Default|GetTarget%20actor)))))
      (:else))))

(event EventBeginPlay
  (CallFunction|BeginInteraction))

(fn GetInteractionUI
  (bind _asbp_hero_controller (Utilities|Casting|CastToBP_HeroController (Game|GetPlayerController 0)))
  (return (Variables|/Game/Player/UI/WB_PlayerHUD.WB_PlayerHUD_C|GetWB_InteractionUI (Variables|/Game/Player/BP_HeroController.BP_HeroController_C|GetPlayerHUD _asbp_hero_controller))))

(fn InteractionTrace
  (bind _returnvalue (Components|GetOwner))
  (bind _returnvalue_2 (Transformation|GetActorLocation _returnvalue))
  (bind (_outhit _returnvalue_3) (Collision|SphereTraceByChannel _returnvalue_2 (+ _returnvalue_2 (* (Transformation|GetActorForwardVector _returnvalue) 1e+02)) 7e+01 "TraceTypeQuery3" false 0 "None"))
  (if _returnvalue_3
    (if (Utilities|DoesObjectImplementInterface (.HitActor (Collision|BreakHitResult _outhit)) "/Game/InteractionSystem/BPI_Interaction.BPI_Interaction_C")
      (bind _output_get (Variables|Default|SetTarget%20actor (.HitActor (Collision|BreakHitResult _outhit))))
      (bind _message (Class|BPIInteraction|Lookat(Message) _output_get))
      (Default|SetMessage (CallFunction|GetInteractionUI) _message)
      (else
        (Variables|Default|SetTarget%20actor 0)
        (Default|SetMessage (CallFunction|GetInteractionUI))))
    (else
      (Variables|Default|SetTarget%20actor 0)
      (Default|SetMessage (CallFunction|GetInteractionUI)))))