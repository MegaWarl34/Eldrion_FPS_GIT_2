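; Item data component that makes its owning actor a pickup for the inventory system.
; On Interact, it passes its item ID and quantity to the PickUp function of the interactor's inventory component, if valid.
; On success it looks up the item's row in DT_ItemData, plays that pickup sound at the owner's location and destroys the owner.
; FocusTarget returns an empty value.
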(event EventBeginPlay)

(event EventTick
  (params (DeltaSeconds :type Float%20%28single-precision%29)))

(event EventInteract
  (params (Interact :type BP%20First%20Person%20Character%20Object%20Reference))
  (bind _bpc_inventory (Variables|/Game/FirstPerson/Blueprints/BP_FirstPersonCharacter.BP_FirstPersonCharacter_C|GetBPC_Inventory Interact)
    (:then
      (bind _sucess (Default|PickUp _bpc_inventory (.RowName (Utilities|Struct|BreakDataTableRowHandle (Variables|Default|GetItemID))) (Variables|Default|GetItemQuantity)))
      (if _sucess
        (bind _returnvalue (Utilities|GetDataTableRow "/Game/Inventory/InventorySystem/ItemData/DT_ItemData.DT_ItemData" (.RowName (Utilities|Struct|BreakDataTableRowHandle (Variables|Default|GetItemID))))
          (:then
            (Audio|PlaySoundatLocation (Utilities|Struct|BreakS_ItemSFX (Utilities|Struct|BreakS_ItemData _returnvalue)) (Transformation|GetActorLocation (Components|GetOwner)) "0, 0, 0" 1.0 1.0 0.0 0 0 0 0)
            (Actor|DestroyActor (Components|GetOwner))))))
    (:else)))

(fn FocusTarget
  (return ""))