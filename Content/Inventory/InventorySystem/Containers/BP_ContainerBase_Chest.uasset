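; BP_ContainerBase_Chest is an inventory container chest whose lid swings open and closed when interacted with.
; OnInteract toggles IsOpen, plays the matching open or close sound from ContainerSFX, and plays or reverses ContainerTimeline.
; The timeline track drives a lerp on the roll of SecondMesh to rotate the lid.
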(event EventBeginPlay
  (|CallParentFunction) ; Ce nœud est désactivé et ne sera pas appelé.\nFaites glisser les broches pour générer des fonctionnalités.
)

(event Collision|EventActorBeginOverlap
  (params (OtherActor :type Actor%20Object%20Reference)))

(event EventTick
  (params (DeltaSeconds :type Float%20%28single-precision%29)))

(event EventOnInteract
  (bind _returnvalue (Transformation|GetActorLocation))
  (bind _containersfx (Variables|Default|GetContainerSFX))
  (bind (_open _close) (Utilities|Struct|BreakS_ContainerSFX _containersfx))
  (if (not (Variables|Default|GetIsOpen))
    (Variables|Default|SetIsOpen true)
    (Audio|PlaySoundatLocation _open _returnvalue "0, 0, 0" 1.0 1.0 0.0 0 0 0 0)
    (bind _container_track (Timeline|ContainerTimeline Play)
      (:Update
        (Transformation|SetRelativeRotation (Variables|Default|GetSecondMesh) (Math|Rotator|MakeRotator (Math|Float|Lerp 0.0 -1.2e+02 _container_track) 0.0 0.0) false false)))
    (else
      (Variables|Default|SetIsOpen false)
      (Audio|PlaySoundatLocation _close _returnvalue "0, 0, 0" 1.0 1.0 0.0 0 0 0 0)
      (Timeline|ContainerTimeline Reverse))))

(fn ConstructionScript
  (|CallParentFunction))