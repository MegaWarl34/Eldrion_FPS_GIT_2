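; Base actor for searchable containers whose inventory component holds item slots and persists through level saves, with a "Search" focus prompt using the container name.
; After a short BeginPlay delay, it restores slots from an existing save or seeds default content.
; Saving appends component and slots to parallel game mode arrays, looked up by component reference on load.
; Interact only casts the player controller; the HUD container display code is disconnected.
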(event Custom|UpdateContainer)

(event EventBeginPlay
  (bind _bpc_inventory (Variables|Default|GetBPC_Inventory))
  (Utilities|FlowControl|Delay 0.2)
  (bind _asbp_first_person_game_mode (Utilities|Casting|CastToBP_FirstPersonGameMode (Game|GetGameMode)))
  (bind _returnvalue (SaveGame|DoesSaveGameExist (Variables|/Game/FirstPerson/Blueprints/BP_FirstPersonGameMode.BP_FirstPersonGameMode_C|GetLevelData _asbp_first_person_game_mode)))
  (if _returnvalue
    (bind _savedata (Class|BPISaveSystems|GetSaveData(Message) (Game|GetGameMode)))
    (Utilities|IsValid (.LevelData (Utilities|Struct|BreakS_SaveData _savedata))
      (:Is%20Valid
        (SaveSystem|LoadContainerData (Variables|/Game/Inventory/InventorySystem/SaveSystem/BP_SaveData_Level.BP_SaveData_Level_C|GetContainersData (.LevelData (Utilities|Struct|BreakS_SaveData _savedata))))))
    (else
      (Variables|/Game/Inventory/InventorySystem/BPC_Inventory.BPC_Inventory_C|SetItemSlots _bpc_inventory (Variables|Default|GetContainerContent))
      (Utilities|Array|Resize (Variables|/Game/Inventory/InventorySystem/BPC_Inventory.BPC_Inventory_C|GetItemSlots _bpc_inventory) (Variables|Default|GetContainerSize)))))

(event EventInteract
  (params (Interact :type BP%20First%20Person%20Character%20Object%20Reference))
  (bind _asbp_mycontroller (Utilities|Casting|CastToBP_Mycontroller (Game|GetPlayerController 0))))

(fn ConstructionScript)

(fn GetContainerData
  (bind _asbp_first_person_game_mode (Utilities|Casting|CastToBP_FirstPersonGameMode (Game|GetGameMode)))
  (Utilities|Array|Add (.Containers (Utilities|Struct|BreakS_ContainerData (Variables|/Game/Inventory/InventorySystem/SaveSystem/BP_SaveData_Level.BP_SaveData_Level_C|GetContainersData (Variables|/Game/FirstPerson/Blueprints/BP_FirstPersonGameMode.BP_FirstPersonGameMode_C|GetSaveDataLevel _asbp_first_person_game_mode)))) (Utilities|ResolveSoftReference (Variables|Default|GetBPC_Inventory)))
  (Utilities|Array|Add (.ContainersInventory (Utilities|Struct|BreakS_ContainerData (Variables|/Game/Inventory/InventorySystem/SaveSystem/BP_SaveData_Level.BP_SaveData_Level_C|GetContainersData (Variables|/Game/FirstPerson/Blueprints/BP_FirstPersonGameMode.BP_FirstPersonGameMode_C|GetSaveDataLevel _asbp_first_person_game_mode)))) (Utilities|Struct|MakeS_ContainerInventory (Variables|/Game/Inventory/InventorySystem/BPC_Inventory.BPC_Inventory_C|GetItemSlots (Variables|Default|GetBPC_Inventory))))
  (return (Variables|/Game/Inventory/InventorySystem/SaveSystem/BP_SaveData_Level.BP_SaveData_Level_C|GetContainersData (Variables|/Game/FirstPerson/Blueprints/BP_FirstPersonGameMode.BP_FirstPersonGameMode_C|GetSaveDataLevel _asbp_first_person_game_mode))))

(fn LoadContainerData
  (params (ContainerData :type S%20Container%20Data%20Structure))
  (bind (_containers _containersinventory) (Utilities|Struct|BreakS_ContainerData ContainerData))
  (bind _output_get (Variables|/Game/Inventory/InventorySystem/BPC_Inventory.BPC_Inventory_C|SetItemSlots (Variables|Default|GetBPC_Inventory) (Utilities|Struct|BreakS_ContainerInventory (Utilities|Array|Get(acopy) _containersinventory (Utilities|Array|FindItem _containers (Utilities|ResolveSoftReference (Variables|Default|GetBPC_Inventory)))))))
  (Utilities|Array|Resize _output_get (Variables|Default|GetContainerSize)))

(fn FocusTarget
  (return (Utilities|Text|FormatText "Search {Container}" (Variables|Default|GetContainerName))))