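; Hotbar inventory component that holds the player's item slots and tracks which of nine is selected.
; On BeginPlay it runs its parent logic, then restores slots from the game instance's save data if a save exists, otherwise refreshes the inventory.
; Numpad keys or wrap-around up/down input actions set the scroll index, which highlights the HUD slot, plays a sound and refreshes the inventory.
; A getter exposes the slot data.
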(event Input|EnhancedActionEvents|EnhancedInputActionIA_HotbarUp
  (params (ActionValue :type Boolean) (ElapsedSeconds :type Float%20%28double-precision%29) (TriggeredSeconds :type Float%20%28double-precision%29) (InputAction :type Input%20Action%20Object%20Reference :default "/Game/FirstPerson/Input/Actions/IA_HotbarUp.IA_HotbarUp"))
  (bind _output_get (Variables|Default|SetScroll%20Index (Math|Integer|Clamp(Integer) (+ (Variables|Default|GetScroll%20Index) 1) -1 9)))
  (if (== _output_get 9)
    (Variables|Default|SetScroll%20Index 0))
  (CallFunction|GetSelectedSlots (Variables|Default|GetScroll%20Index)))

(event Input|EnhancedActionEvents|EnhancedInputActionIA_HotbarDown
  (params (ActionValue :type Boolean) (ElapsedSeconds :type Float%20%28double-precision%29) (TriggeredSeconds :type Float%20%28double-precision%29) (InputAction :type Input%20Action%20Object%20Reference :default "/Game/FirstPerson/Input/Actions/IA_HotbarDown.IA_HotbarDown"))
  (bind _output_get (Variables|Default|SetScroll%20Index (Math|Integer|Clamp(Integer) (- (Variables|Default|GetScroll%20Index) 1) -1 9)))
  (if (== _output_get -1)
    (Variables|Default|SetScroll%20Index 8))
  (CallFunction|GetSelectedSlots (Variables|Default|GetScroll%20Index)))

(event EventBeginPlay
  (|CallParentFunction)
  (bind _returnvalue (SaveGame|DoesSaveGameExist "slot1"))
  (if _returnvalue
    (bind _savedata (Class|BPISaveSystems|GetSaveData(Message) (Game|GetGameInstance)))
    (Utilities|IsValid (.PlayerData (Utilities|Struct|BreakS_SaveData _savedata))
      (:Is%20Valid
        (SaveSystem|LoadHotbarData (Variables|/Game/Inventory/InventorySystem/SaveSystem/BP_SaveDataPlayer.BP_SaveDataPlayer_C|GetHotbarData (.PlayerData (Utilities|Struct|BreakS_SaveData _savedata))))))
    (else
      (CallFunction|UpdateInventory))))

(event EventTick
  (params (DeltaSeconds :type Float%20%28single-precision%29)))

(event Input|KeyboardEvents|NumPadNine
  (params (Key :type Key%20Structure :default "None"))
  (:Pressed
    (bind _output_get (Variables|Default|SetScroll%20Index 8))
    (CallFunction|GetSelectedSlots _output_get)))

(event Input|KeyboardEvents|NumPadOne
  (params (Key :type Key%20Structure :default "None"))
  (:Pressed
    (bind _output_get (Variables|Default|SetScroll%20Index 0))
    (CallFunction|GetSelectedSlots _output_get)))

(event Input|KeyboardEvents|NumPadTwo
  (params (Key :type Key%20Structure :default "None"))
  (:Pressed
    (bind _output_get (Variables|Default|SetScroll%20Index 1))
    (CallFunction|GetSelectedSlots _output_get)))

(event Input|KeyboardEvents|NumPadThree
  (params (Key :type Key%20Structure :default "None"))
  (:Pressed
    (bind _output_get (Variables|Default|SetScroll%20Index 2))
    (CallFunction|GetSelectedSlots _output_get)))

(event Input|KeyboardEvents|NumPadFour
  (params (Key :type Key%20Structure :default "None"))
  (:Pressed
    (bind _output_get (Variables|Default|SetScroll%20Index 3))
    (CallFunction|GetSelectedSlots _output_get)))

(event Input|KeyboardEvents|NumPadFive
  (params (Key :type Key%20Structure :default "None"))
  (:Pressed
    (bind _output_get (Variables|Default|SetScroll%20Index 4))
    (CallFunction|GetSelectedSlots _output_get)))

(event Input|KeyboardEvents|NumPadSix
  (params (Key :type Key%20Structure :default "None"))
  (:Pressed
    (bind _output_get (Variables|Default|SetScroll%20Index 5))
    (CallFunction|GetSelectedSlots _output_get)))

(event Input|KeyboardEvents|NumPadSeven
  (params (Key :type Key%20Structure :default "None"))
  (:Pressed
    (bind _output_get (Variables|Default|SetScroll%20Index 6))
    (CallFunction|GetSelectedSlots _output_get)))

(event Input|KeyboardEvents|NumPadEight
  (params (Key :type Key%20Structure :default "None"))
  (:Pressed
    (bind _output_get (Variables|Default|SetScroll%20Index 7))
    (CallFunction|GetSelectedSlots _output_get)))

(fn GetSelectedSlots
  (params (Index :type Integer))
  (bind _itemslots (Variables|Default|GetItemSlots))
  (bind _output (Utilities|Array|Get(acopy) _itemslots Index))
  (LocalVariables|SetLocal%20Item%20ID (.itemid _output))
  (LocalVariables|SetLocal%20Item%20Quantity (.itemquantity _output))
  (Default|SelectedSlots (Variables|/Game/Inventory/WB_PlayerHUD.WB_PlayerHUD_C|GetWb_HotbarDisplay (CallFunction|GetPlayerHUD)) Index)
  (Audio|PlaySoundatLocation 0 (Transformation|GetActorLocation (Components|GetOwner)) "0, 0, 0" 1.0 1.0 0.0 0 0 0 0)
  (CallFunction|UpdateInventory)
  (return Index))

(fn LoadHotbarData
  (params (HotbarData :type Array%20of%20S-Item%20Slot%20Structures))
  (Variables|Default|SetItemSlots HotbarData)
  (Utilities|Array|Resize (Variables|Default|GetItemSlots) (Variables|Default|GetInventorysize))
  (CallFunction|UpdateInventory))

(fn GetHotbarData
  (return (Variables|Default|GetItemSlots)))