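; BP_ContainerBase is a lootable container actor with an inventory component, a "Search" look-at prompt and persistent contents.
; BeginPlay waits briefly, then restores slots from the level save or fills them from defaults.
; Interacting opens the inventory UI through the hero controller, while a separate toggle plays open/close sounds and drives a timeline-based lid rotation.
; Saving appends to parallel arrays in game-mode level data, matched on load by inventory component reference.
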(event Custom|UpdateAnimation
  (bind _returnvalue (Transformation|GetActorLocation))
  (bind _containersfx (Variables|Default|GetContainerSFX))
  (bind (_open _close) (Utilities|Struct|BreakS_ContainerSFX _containersfx))
  (if (not (Variables|Default|GetIsOpen))
    (Variables|Default|SetIsOpen true)
    (Audio|PlaySoundatLocation _open _returnvalue "0, 0, 0" 1.0 1.0 0.0 0 0 0 0)
    (else
      (Variables|Default|SetIsOpen false)
      (Audio|PlaySoundatLocation _close _returnvalue "0, 0, 0" 1.0 1.0 0.0 0 0 0 0)
      (bind _nouvelle_piste_0 (Timeline|ContainerTimeline Reverse)
        (:Update
          (Transformation|SetRelativeRotation (Variables|Default|GetContainerLid) (Math|Rotator|MakeRotator (Math|Float|Lerp 0.0 -1.2e+02 _nouvelle_piste_0) 0.0 0.0) false false))))))

(event EventBeginPlay
  (bind _bpc_inventory (Variables|Default|GetBPC_Inventory))
  (Utilities|FlowControl|Delay 0.2)
  (bind _asbp_third_person_game_mode (Utilities|Casting|CastToBP_ThirdPersonGameMode (Game|GetGameMode)))
  (bind _returnvalue (SaveGame|DoesSaveGameExist (Variables|/Game/ThirdPerson/Blueprints/BP_ThirdPersonGameMode.BP_ThirdPersonGameMode_C|GetLevelData _asbp_third_person_game_mode)))
  (if _returnvalue
    (bind _gamedata (Class|BPISaveSystem|GetGameData(Message) (Game|GetGameMode)))
    (Utilities|IsValid (.LevelData (Utilities|Struct|BreakS_GameData _gamedata))
      (:Is%20Valid
        (CallFunction|LoadContainerData (Variables|/Game/SaveSystem/SGB_LevelData.SGB_LevelData_C|GetContainerData (.LevelData (Utilities|Struct|BreakS_GameData _gamedata))))))
    (else
      (Variables|/Game/Inventory_System/BPC_Inventory.BPC_Inventory_C|SetItemSlots _bpc_inventory (Variables|Default|GetContainerSlots))
      (Utilities|Array|Resize (Variables|/Game/Inventory_System/BPC_Inventory.BPC_Inventory_C|GetItemSlots _bpc_inventory) (Variables|Default|GetContainerSize)))))

(event EventInteractwith
  (params (Interactor :type Actor%20Object%20Reference))
  (bind _asbp_hero_controller (Utilities|Casting|CastToBP_HeroController (Game|GetPlayerController 0)))
  (bind _inventoryactor (Default|CreateInventoryActor _asbp_hero_controller))
  (bind _containerdisplay (Default|OpenContainer _inventoryactor (Variables|Default|GetBPC_Inventory)))
  (EventDispatchers|BindEventtoOnContainerClosed _containerdisplay (EventDispatchers|CreateEvent :!event Custom|UpdateAnimation))
  (Development|PrintString "Container Open"))

(event EventInteractAction
  (bind _returnvalue (Transformation|GetActorLocation))
  (bind _containersfx (Variables|Default|GetContainerSFX))
  (bind (_open _close) (Utilities|Struct|BreakS_ContainerSFX _containersfx))
  (if (not (Variables|Default|GetIsOpen))
    (Variables|Default|SetIsOpen true)
    (Audio|PlaySoundatLocation _open _returnvalue "0, 0, 0" 1.0 1.0 0.0 0 0 0 0)
    (else
      (Variables|Default|SetIsOpen false)
      (Audio|PlaySoundatLocation _close _returnvalue "0, 0, 0" 1.0 1.0 0.0 0 0 0 0)
      (bind _nouvelle_piste_0 (Timeline|ContainerTimeline Reverse)
        (:Update
          (Transformation|SetRelativeRotation (Variables|Default|GetContainerLid) (Math|Rotator|MakeRotator (Math|Float|Lerp 0.0 -1.2e+02 _nouvelle_piste_0) 0.0 0.0) false false))))))

(fn ConstructionScript)

(fn GetContainerData
  (bind _asbp_third_person_game_mode (Utilities|Casting|CastToBP_ThirdPersonGameMode (Game|GetGameMode)))
  (Utilities|Array|Add (.Containers (Utilities|Struct|BreakS_ContainerData (Variables|/Game/SaveSystem/SGB_LevelData.SGB_LevelData_C|GetContainerData (Variables|/Game/ThirdPerson/Blueprints/BP_ThirdPersonGameMode.BP_ThirdPersonGameMode_C|GetSGB_LevelData _asbp_third_person_game_mode)))) (Utilities|ResolveSoftReference (Variables|Default|GetBPC_Inventory)))
  (Utilities|Array|Add (.ContainerInventory (Utilities|Struct|BreakS_ContainerData (Variables|/Game/SaveSystem/SGB_LevelData.SGB_LevelData_C|GetContainerData (Variables|/Game/ThirdPerson/Blueprints/BP_ThirdPersonGameMode.BP_ThirdPersonGameMode_C|GetSGB_LevelData _asbp_third_person_game_mode)))) (Utilities|Struct|MakeS_ContainerInventory (Variables|/Game/Inventory_System/BPC_Inventory.BPC_Inventory_C|GetItemSlots (Variables|Default|GetBPC_Inventory))))
  (return (Variables|/Game/SaveSystem/SGB_LevelData.SGB_LevelData_C|GetContainerData (Variables|/Game/ThirdPerson/Blueprints/BP_ThirdPersonGameMode.BP_ThirdPersonGameMode_C|GetSGB_LevelData _asbp_third_person_game_mode))))

(fn LoadContainerData
  (params (ContainerData :type S%20Container%20Data%20Structure))
  (bind (_containers _containerinventory) (Utilities|Struct|BreakS_ContainerData ContainerData))
  (bind _output_get (Variables|/Game/Inventory_System/BPC_Inventory.BPC_Inventory_C|SetItemSlots (Variables|Default|GetBPC_Inventory) (Utilities|Struct|BreakS_ContainerInventory (Utilities|Array|Get(acopy) _containerinventory (Utilities|Array|FindItem _containers (Utilities|ResolveSoftReference (Variables|Default|GetBPC_Inventory)))))))
  (Utilities|Array|Resize _output_get (Variables|Default|GetContainerSize)))

(fn Lookat
  (return (Utilities|Text|FormatText "Search {X}" (Variables|Default|GetContainerName))))