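; Player stats component for BP_FirstPersonCharacter that tracks health, stamina, XP and level.
; BeginPlay waits a tick, caches the owner and fills its HUD widget, though the initial health bar is computed from CurrentStamina.
; Each stat function updates the HUD directly; health and stamina gains clamp to max, and decreases return true when depleted.
; Reaching MaxXP raises the level, increases the threshold and resets XP, discarding overflow.
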(event EventBeginPlay
  (Utilities|FlowControl|DelayUntilNextTick)
  (bind _asbp_first_person_character (Utilities|Casting|CastToBP_FirstPersonCharacter (Components|GetOwner)))
  (Variables|Default|SetPlayer%20Character%20BP _asbp_first_person_character)
  (Progress|SetPercent (Variables|/Game/Blueprints/UI/WB_HUD_NEW.WB_HUD_NEW_C|GetStamina_Bar (Variables|/Game/FirstPerson/Blueprints/BP_FirstPersonCharacter.BP_FirstPersonCharacter_C|GetHUD%20Widget%20New (Variables|Default|GetPlayer%20Character%20BP))) (/ (Variables|Stamina|GetCurrent%20Stamina) (Variables|Stamina|GetMax%20Stamina)))
  (Progress|SetPercent (Variables|/Game/Blueprints/UI/WB_HUD_NEW.WB_HUD_NEW_C|GetHealth_Bar (Variables|/Game/FirstPerson/Blueprints/BP_FirstPersonCharacter.BP_FirstPersonCharacter_C|GetHUD%20Widget%20New (Variables|Default|GetPlayer%20Character%20BP))) (/ (Variables|Stamina|GetCurrent%20Stamina) (Variables|Health|GetMax%20Health)))
  (Rendering|Components|TextRender|SetText (Variables|/Game/Blueprints/UI/WB_HUD_NEW.WB_HUD_NEW_C|GetHealth_Text (Variables|/Game/FirstPerson/Blueprints/BP_FirstPersonCharacter.BP_FirstPersonCharacter_C|GetHUD%20Widget%20New (Variables|Default|GetPlayer%20Character%20BP))) (Utilities|Text|ToText(Float) (Variables|Health|GetCurrent%20Health) "HalfToEven"))
  (Progress|SetPercent (Variables|/Game/Blueprints/UI/WB_HUD_NEW.WB_HUD_NEW_C|GetXP_Bar (Variables|/Game/FirstPerson/Blueprints/BP_FirstPersonCharacter.BP_FirstPersonCharacter_C|GetHUD%20Widget%20New (Variables|Default|GetPlayer%20Character%20BP))) (/ (Variables|XP|GetXP) (Variables|XP|GetMax%20XP)))
  (Rendering|Components|TextRender|SetText (Variables|/Game/Blueprints/UI/WB_HUD_NEW.WB_HUD_NEW_C|GetXP_Text (Variables|/Game/FirstPerson/Blueprints/BP_FirstPersonCharacter.BP_FirstPersonCharacter_C|GetHUD%20Widget%20New (Variables|Default|GetPlayer%20Character%20BP))) (Utilities|Text|FormatText "{Current XP} / {Max XP}" (Variables|XP|GetXP) (Variables|XP|GetMax%20XP)))
  (Rendering|Components|TextRender|SetText (Variables|/Game/Blueprints/UI/WB_HUD_NEW.WB_HUD_NEW_C|GetLevel_Text (Variables|/Game/FirstPerson/Blueprints/BP_FirstPersonCharacter.BP_FirstPersonCharacter_C|GetHUD%20Widget%20New (Variables|Default|GetPlayer%20Character%20BP))) (Utilities|Text|ToText(Integer) (Variables|XP|GetLevel))))

(fn DecreaseHealth
  (params (Damage :type Float%20%28double-precision%29))
  (bind _player_character_bp (Variables|Default|GetPlayer%20Character%20BP))
  (bind _hud_widget_new (Variables|/Game/FirstPerson/Blueprints/BP_FirstPersonCharacter.BP_FirstPersonCharacter_C|GetHUD%20Widget%20New _player_character_bp))
  (if (not (<= (Variables|Health|GetCurrent%20Health) 0.0))
    (bind _output_get (Variables|Health|SetCurrent%20Health (- (Variables|Health|GetCurrent%20Health) Damage)))
    (Progress|SetPercent (Variables|/Game/Blueprints/UI/WB_HUD_NEW.WB_HUD_NEW_C|GetHealth_Bar _hud_widget_new) (/ _output_get (Variables|Health|GetMax%20Health)))
    (Rendering|Components|TextRender|SetText (Variables|/Game/Blueprints/UI/WB_HUD_NEW.WB_HUD_NEW_C|GetHealth_Text _hud_widget_new) (Utilities|Text|ToText(Float) (Variables|Health|GetCurrent%20Health) "HalfToEven"))
    (if (<= (Variables|Health|GetCurrent%20Health) 0.0)
      _
      (else
        (return false))))
  (return true))

(fn IncreaseMaxHealth
  (params (Health%20adding :type Float%20%28double-precision%29))
  (bind _player_character_bp (Variables|Default|GetPlayer%20Character%20BP))
  (bind _hud_widget_new (Variables|/Game/FirstPerson/Blueprints/BP_FirstPersonCharacter.BP_FirstPersonCharacter_C|GetHUD%20Widget%20New _player_character_bp))
  (Variables|Health|SetMax%20Health (+ (Variables|Health|GetMax%20Health) Health%20adding))
  (Progress|SetPercent (Variables|/Game/Blueprints/UI/WB_HUD_NEW.WB_HUD_NEW_C|GetHealth_Bar _hud_widget_new) (/ (Variables|Health|GetCurrent%20Health) (Variables|Health|GetMax%20Health)))
  (Rendering|Components|TextRender|SetText (Variables|/Game/Blueprints/UI/WB_HUD_NEW.WB_HUD_NEW_C|GetHealth_Text _hud_widget_new) (Utilities|Text|ToText(Float) (Variables|Health|GetCurrent%20Health) "HalfToEven")))

(fn DecreaseStamina
  (params (Stamina%20Use :type Float%20%28double-precision%29))
  (if (not (<= (Variables|Stamina|GetCurrent%20Stamina) 0.0))
    (Variables|Stamina|SetCurrent%20Stamina (- (Variables|Stamina|GetCurrent%20Stamina) Stamina%20Use))
    (Progress|SetPercent (Variables|/Game/Blueprints/UI/WB_HUD_NEW.WB_HUD_NEW_C|GetStamina_Bar (Variables|/Game/FirstPerson/Blueprints/BP_FirstPersonCharacter.BP_FirstPersonCharacter_C|GetHUD%20Widget%20New (Variables|Default|GetPlayer%20Character%20BP))) (/ (Variables|Stamina|GetCurrent%20Stamina) (Variables|Stamina|GetMax%20Stamina)))
    (if (<= (Variables|Stamina|GetCurrent%20Stamina) 0.0)
      _
      (else
        (return false))))
  (return true))

(fn IncreaseMaxStamina
  (params (Added%20Stamina :type Float%20%28double-precision%29))
  (Variables|Stamina|SetMax%20Stamina (+ (Variables|Stamina|GetMax%20Stamina) Added%20Stamina))
  (Progress|SetPercent (Variables|/Game/Blueprints/UI/WB_HUD_NEW.WB_HUD_NEW_C|GetStamina_Bar (Variables|/Game/FirstPerson/Blueprints/BP_FirstPersonCharacter.BP_FirstPersonCharacter_C|GetHUD%20Widget%20New (Variables|Default|GetPlayer%20Character%20BP))) (/ (Variables|Stamina|GetCurrent%20Stamina) (Variables|Stamina|GetMax%20Stamina))))

(fn IncreaseHealth
  (params (Added%20Health :type Float%20%28double-precision%29))
  (bind _player_character_bp (Variables|Default|GetPlayer%20Character%20BP))
  (bind _hud_widget_new (Variables|/Game/FirstPerson/Blueprints/BP_FirstPersonCharacter.BP_FirstPersonCharacter_C|GetHUD%20Widget%20New _player_character_bp))
  (Variables|Health|SetCurrent%20Health (+ (Variables|Health|GetCurrent%20Health) Added%20Health))
  (if (> (Variables|Health|GetCurrent%20Health) (Variables|Health|GetMax%20Health))
    (Variables|Health|SetCurrent%20Health (Variables|Health|GetMax%20Health)))
  (Progress|SetPercent (Variables|/Game/Blueprints/UI/WB_HUD_NEW.WB_HUD_NEW_C|GetHealth_Bar _hud_widget_new) (/ (Variables|Health|GetCurrent%20Health) (Variables|Health|GetMax%20Health)))
  (Rendering|Components|TextRender|SetText (Variables|/Game/Blueprints/UI/WB_HUD_NEW.WB_HUD_NEW_C|GetHealth_Text _hud_widget_new) (Utilities|Text|ToText(Float) (Variables|Health|GetCurrent%20Health) "HalfToEven")))

(fn RegenStamina
  (params (Added%20Stamina :type Float%20%28double-precision%29))
  (Variables|Stamina|SetCurrent%20Stamina (+ (Variables|Stamina|GetCurrent%20Stamina) Added%20Stamina))
  (if (> (Variables|Stamina|GetCurrent%20Stamina) (Variables|Stamina|GetMax%20Stamina))
    (Variables|Stamina|SetCurrent%20Stamina (Variables|Stamina|GetMax%20Stamina)))
  (Progress|SetPercent (Variables|/Game/Blueprints/UI/WB_HUD_NEW.WB_HUD_NEW_C|GetStamina_Bar (Variables|/Game/FirstPerson/Blueprints/BP_FirstPersonCharacter.BP_FirstPersonCharacter_C|GetHUD%20Widget%20New (Variables|Default|GetPlayer%20Character%20BP))) (/ (Variables|Stamina|GetCurrent%20Stamina) (Variables|Stamina|GetMax%20Stamina))))

(fn IncreaseXP
  (params (Added%20Xp :type Float%20%28double-precision%29))
  (Variables|XP|SetXP (+ (Variables|XP|GetXP) Added%20Xp))
  (if (>= (Variables|XP|GetXP) (Variables|XP|GetMax%20XP))
    (XPAndLevel|IncreaseLevel 1))
  (Progress|SetPercent (Variables|/Game/Blueprints/UI/WB_HUD_NEW.WB_HUD_NEW_C|GetXP_Bar (Variables|/Game/FirstPerson/Blueprints/BP_FirstPersonCharacter.BP_FirstPersonCharacter_C|GetHUD%20Widget%20New (Variables|Default|GetPlayer%20Character%20BP))) (/ (Variables|XP|GetXP) (Variables|XP|GetMax%20XP)))
  (Rendering|Components|TextRender|SetText (Variables|/Game/Blueprints/UI/WB_HUD_NEW.WB_HUD_NEW_C|GetXP_Text (Variables|/Game/FirstPerson/Blueprints/BP_FirstPersonCharacter.BP_FirstPersonCharacter_C|GetHUD%20Widget%20New (Variables|Default|GetPlayer%20Character%20BP))) (Utilities|Text|FormatText "{Current XP} / {Max XP}" (Variables|XP|GetXP) (Variables|XP|GetMax%20XP))))

(fn IncreaseLevel
  (params (Added%20Level :type Integer))
  (Variables|XP|SetLevel (+ (Variables|XP|GetLevel) Added%20Level))
  (Variables|XP|SetMax%20XP (+ (Variables|XP|GetMax%20XP) 1.5e+02))
  (Variables|XP|SetXP 0.0)
  (Rendering|Components|TextRender|SetText (Variables|/Game/Blueprints/UI/WB_HUD_NEW.WB_HUD_NEW_C|GetLevel_Text (Variables|/Game/FirstPerson/Blueprints/BP_FirstPersonCharacter.BP_FirstPersonCharacter_C|GetHUD%20Widget%20New (Variables|Default|GetPlayer%20Character%20BP))) (Utilities|Text|ToText(Integer) (Variables|XP|GetLevel))))