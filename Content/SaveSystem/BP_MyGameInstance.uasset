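; Game instance that owns the player's save data and persists it to a single save slot.
; On init it loads the existing slot into an SGB_PlayerData object, or creates a new one if none exists.
; SavePlayerData copies inventory, hotbar and character equipment into that object and writes it to disk immediately.
; GetGameData returns the held save object wrapped in an SGameData struct.
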(event EventInit
  (CallFunction|LoadGameData))

(event EventLoadGameData
  (bind _returnvalue (SaveGame|DoesSaveGameExist "Slot1"))
  (if _returnvalue
    (bind _returnvalue_2 (SaveGame|LoadGamefromSlot "Slot1"))
    (bind _assgb_player_data (Utilities|Casting|CastToSGB_PlayerData _returnvalue_2))
    (Variables|Default|SetBP_PlayerData _assgb_player_data)
    (else
      (bind _returnvalue_3 (SaveGame|CreateSaveGameObject "/Game/SaveSystem/SGB_PlayerData.SGB_PlayerData_C"))
      (Variables|Default|SetBP_PlayerData _returnvalue_3))))

(event EventSaveGameData
  (SaveGame|SaveGametoSlot (Variables|Default|GetBP_PlayerData) "Slot1"))

(event EventSavePlayerData
  (params (InventoryData :type Array%20of%20S%20Item%20Slots%20Structures) (HotbarData :type Array%20of%20S%20Item%20Slots%20Structures) (CharacterEquipment :type Array%20of%20S%20Item%20Slots%20Structures))
  (Variables|/Game/SaveSystem/SGB_PlayerData.SGB_PlayerData_C|SetInventoryData (Variables|Default|GetBP_PlayerData) InventoryData)
  (Variables|/Game/SaveSystem/SGB_PlayerData.SGB_PlayerData_C|SetHotBarData (Variables|Default|GetBP_PlayerData) HotbarData)
  (Variables|/Game/SaveSystem/SGB_PlayerData.SGB_PlayerData_C|SetCharacterEquipment (Variables|Default|GetBP_PlayerData) CharacterEquipment)
  (CallFunction|SaveGameData))

(fn GetGameData
  (return (Utilities|Struct|MakeS_GameData (Variables|Default|GetBP_PlayerData))))