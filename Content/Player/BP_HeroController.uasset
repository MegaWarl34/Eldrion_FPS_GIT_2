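; Hero controller that shows the player HUD, autosaves player and level data on a looping one-second timer, and handles inventory input.
; The inventory action closes an open container or the inventory, or creates and opens a new inventory when none exists.
; Creating an inventory first spawns a wardrobe actor far above the world origin, then spawns the inventory actor at that transform with the wardrobe passed in.
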(event Custom|autosave
  (CallFunction|SavePlayerData)
  (CallFunction|SaveLevelData))

(event Input|EnhancedActionEvents|EnhancedInputActionIA_Inventory
  (params (ActionValue :type Boolean) (ElapsedSeconds :type Float%20%28double-precision%29) (TriggeredSeconds :type Float%20%28double-precision%29) (InputAction :type Input%20Action%20Object%20Reference :default "/Game/ThirdPerson/Input/Actions/IA_Inventory.IA_Inventory"))
  (:Started
    (bind _inventoryactor (Variables|Default|GetInventoryActor)
      (:then
        (Variables|/Game/Inventory_System/InventoryActor/BP_InventoryActor.BP_InventoryActor_C|GetContainerDisplay _inventoryactor
          (:then
            (Default|CloseContainer (Variables|Default|GetInventoryActor))
            (Development|PrintString "Container Close"))
          (:else)))
      (:else))))

(event Input|EnhancedActionEvents|EnhancedInputActionIA_Inventory
  (params (ActionValue :type Boolean) (ElapsedSeconds :type Float%20%28double-precision%29) (TriggeredSeconds :type Float%20%28double-precision%29) (InputAction :type Input%20Action%20Object%20Reference :default "/Game/ThirdPerson/Input/Actions/IA_Inventory.IA_Inventory"))
  (:Started
    (bind _inventoryactor (Variables|Default|GetInventoryActor)
      (:then
        (Variables|/Game/Inventory_System/InventoryActor/BP_InventoryActor.BP_InventoryActor_C|GetContainerDisplay _inventoryactor
          (:then
            (Default|CloseContainer (Variables|Default|GetInventoryActor))
            (Development|PrintString "Container Close"))
          (:else
            (Default|CloseInventory (Variables|Default|GetInventoryActor))
            (Development|PrintString "Inventory close"))))
      (:else
        (bind _inventoryactor_2 (CallFunction|CreateInventoryActor))
        (Default|OpenInventory _inventoryactor_2)
        (Development|PrintString "Inventory open")))))

(event EventBeginPlay
  (Utilities|FlowControl|Sequence
    (:then_0
      (CallFunction|ShowPlayerHUD))
    (:then_1
      (Utilities|Time|SetTimerbyEvent (delegate Custom|autosave) 1.0 true))))

(fn ConstructionScript)

(fn ShowPlayerHUD
  (bind _returnvalue (UserInterface|CreateWidget "/Game/Player/UI/WB_PlayerHUD.WB_PlayerHUD_C"))
  (bind _output_get (Variables|Default|SetPlayerHUD _returnvalue))
  (UserInterface|Viewport|AddtoViewport _output_get 0))

(fn CreateWardrobeActor
  (bind _returnvalue (Game|SpawnActorfromClass "/Game/Inventory_System/InventoryActor/BP_WardrobeActor.BP_WardrobeActor_C" (Math|Transform|MakeTransform "0.000000,0.000000,1000000.000000" "0, 0, 0" "1.000000,1.000000,1.000000") "AlwaysSpawn" "MultiplyWithRoot" 0 0))
  (bind _output_get (Variables|Default|SetWardRobeActor _returnvalue))
  (return (Transformation|GetActorTransform _output_get) (Variables|Default|GetWardRobeActor)))

(fn CreateInventoryActor
  (bind (_transform _wardrobeactor) (CallFunction|CreateWardrobeActor))
  (bind _returnvalue (Game|SpawnActorfromClass "/Game/Inventory_System/InventoryActor/BP_InventoryActor.BP_InventoryActor_C" _transform "Undefined" "MultiplyWithRoot" 0 _wardrobeactor 0))
  (bind _output_get (Variables|Default|SetInventoryActor _returnvalue))
  (return _output_get))