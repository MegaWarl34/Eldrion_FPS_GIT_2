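; Hotbar component of the inventory system, letting the player select one of nine slots with numpad keys or the mouse wheel, which wraps around.
; Selection caches the slot's item ID and quantity, highlights it on the HUD, plays a sound and refreshes the inventory.
; On BeginPlay it restores slots from the game instance's player data when save "Slot1" exists, and exposes them through GetHotbarData.
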(event EventTick
  (params (DeltaSeconds :type Float%20%28single-precision%29)))

(event EventBeginPlay
  (|CallParentFunction)
  (bind _returnvalue (SaveGame|DoesSaveGameExist "Slot1"))
  (if _returnvalue
    (bind _gamedata (Class|BPISaveSystem|GetGameData(Message) (Game|GetGameInstance)))
    (Utilities|IsValid (.PlayerData (Utilities|Struct|BreakS_GameData _gamedata))
      (:Is%20Valid
        (CallFunction|LoadHotBarData (Variables|/Game/SaveSystem/SGB_PlayerData.SGB_PlayerData_C|GetHotBarData (.PlayerData (Utilities|Struct|BreakS_GameData _gamedata))))))
    (else
      (CallFunction|UpdateInventory))))

(event Input|KeyboardEvents|NumPadNine
  (params (Key :type Key%20Structure :default "None"))
  (:Pressed
    (bind _output_get (Variables|Default|SetScroll%20Index 8))
    (CallFunction|GetSelectedSlot _output_get)))

(event Input|KeyboardEvents|NumPadOne
  (params (Key :type Key%20Structure :default "None"))
  (:Pressed
    (bind _output_get (Variables|Default|SetScroll%20Index 0))
    (CallFunction|GetSelectedSlot _output_get)))

(event Input|MouseEvents|MouseWheelDown
  (params (Key :type Key%20Structure :default "None"))
  (:Pressed
    (bind _output_get (Variables|Default|SetScroll%20Index (Math|Integer|Clamp(Integer) (- (Variables|Default|GetScroll%20Index) 1) -1 9)))
    (if (== _output_get -1)
      (Variables|Default|SetScroll%20Index 8))
    (CallFunction|GetSelectedSlot (Variables|Default|GetScroll%20Index))))

(event Input|KeyboardEvents|NumPadTwo
  (params (Key :type Key%20Structure :default "None"))
  (:Pressed
    (bind _output_get (Variables|Default|SetScroll%20Index 1))
    (CallFunction|GetSelectedSlot _output_get)))

(event Input|KeyboardEvents|NumPadThree
  (params (Key :type Key%20Structure :default "None"))
  (:Pressed
    (bind _output_get (Variables|Default|SetScroll%20Index 2))
    (CallFunction|GetSelectedSlot _output_get)))

(event Input|KeyboardEvents|NumPadFour
  (params (Key :type Key%20Structure :default "None"))
  (:Pressed
    (bind _output_get (Variables|Default|SetScroll%20Index 3))
    (CallFunction|GetSelectedSlot _output_get)))

(event Input|KeyboardEvents|NumPadFive
  (params (Key :type Key%20Structure :default "None"))
  (:Pressed
    (bind _output_get (Variables|Default|SetScroll%20Index 4))
    (CallFunction|GetSelectedSlot _output_get)))

(event Input|KeyboardEvents|NumPadSix
  (params (Key :type Key%20Structure :default "None"))
  (:Pressed
    (bind _output_get (Variables|Default|SetScroll%20Index 5))
    (CallFunction|GetSelectedSlot _output_get)))

(event Input|KeyboardEvents|NumPadSeven
  (params (Key :type Key%20Structure :default "None"))
  (:Pressed
    (bind _output_get (Variables|Default|SetScroll%20Index 6))
    (CallFunction|GetSelectedSlot _output_get)))

(event Input|KeyboardEvents|NumPadEight
  (params (Key :type Key%20Structure :default "None"))
  (:Pressed
    (bind _output_get (Variables|Default|SetScroll%20Index 7))
    (CallFunction|GetSelectedSlot _output_get)))

(event Input|MouseEvents|MouseWheelUp
  (params (Key :type Key%20Structure :default "None"))
  (:Pressed
    (bind _output_get (Variables|Default|SetScroll%20Index (Math|Integer|Clamp(Integer) (+ (Variables|Default|GetScroll%20Index) 1) -1 9)))
    (if (== _output_get 9)
      (Variables|Default|SetScroll%20Index 0))
    (CallFunction|GetSelectedSlot (Variables|Default|GetScroll%20Index))))

(fn GetSelectedSlot
  (params (Index :type Integer))
  (bind _itemslots (Variables|Default|GetItemSlots))
  (bind _output (Utilities|Array|Get(acopy) _itemslots Index))
  (LocalVariables|SetLocal_ItemID (.itemid _output))
  (LocalVariables|SetLocal_ItemQuantity (.itemquantity _output))
  (Default|SetSelectedSlot (Variables|/Game/Player/UI/WB_PlayerHUD.WB_PlayerHUD_C|GetWB_HotbarDisplay (CallFunction|GetPlayerHud)) Index)
  (Audio|PlaySound2D 0 1.0 1.0 0.0 0 0)
  (CallFunction|UpdateInventory))

(fn GetHotbarData
  (return (Variables|Default|GetItemSlots)))

(fn LoadHotBarData
  (params (ItemSlots :type Array%20of%20S%20Item%20Slots%20Structures))
  (Variables|Default|SetItemSlots ItemSlots)
  (Utilities|Array|Resize (Variables|Default|GetItemSlots) (Variables|Default|GetInventorySize))
  (CallFunction|UpdateInventory))