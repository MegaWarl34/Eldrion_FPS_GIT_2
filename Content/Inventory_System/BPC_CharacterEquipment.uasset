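; BPC_CharacterEquipment is a component that holds the character's equipment slots and restores them from saved game data.
; On BeginPlay it runs the parent logic, then, if save "Slot1" exists, gets PlayerData through the GameInstance and loads its CharacterEquipment.
; Loading replaces ItemSlots, resizes it to InventorySize and calls EquipItem.
; GetEquipmentData exposes the current slots.
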(event EventTick
  (params (DeltaSeconds :type Float%20%28single-precision%29)))

(event EventBeginPlay
  (|CallParentFunction)
  (bind _returnvalue (SaveGame|DoesSaveGameExist "Slot1"))
  (if _returnvalue
    (bind _gamedata (Class|BPISaveSystem|GetGameData(Message) (Game|GetGameInstance)))
    (Utilities|IsValid (.PlayerData (Utilities|Struct|BreakS_GameData _gamedata))
      (:Is%20Valid
        (CallFunction|LoadEquipmentData (Variables|/Game/SaveSystem/SGB_PlayerData.SGB_PlayerData_C|GetCharacterEquipment (.PlayerData (Utilities|Struct|BreakS_GameData _gamedata))))))))

(fn GetEquipmentData
  (return (Variables|Default|GetItemSlots)))

(fn LoadEquipmentData
  (params (ItemSlots :type Array%20of%20S%20Item%20Slots%20Structures))
  (bind _output_get (Variables|Default|SetItemSlots ItemSlots))
  (Utilities|Array|Resize _output_get (Variables|Default|GetInventorySize))
  (CallFunction|EquipItem))