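; BP_InventoryActor is a temporary actor that backs the inventory and container screens with a scene capture of the Wardrobe actor.
; Opening either screen limits the capture to Wardrobe, adds the player or container widget and moves input from the hero to this actor.
; Mouse input drives the spring arm: left-drag rotates, wheel zooms within limits and right-click resets.
; Closing removes the widget, returns input to the hero and destroys the actor.
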(event EventBeginPlay)

(event Collision|EventActorBeginOverlap
  (params (OtherActor :type Actor%20Object%20Reference)))

(event EventTick
  (params (DeltaSeconds :type Float%20%28single-precision%29)))

(event Input|MouseEvents|MouseX
  (params (AxisValue :type Float%20%28single-precision%29))
  (if (Variables|Default|GetShouldRotated)
    (Transformation|SetWorldRotation (Variables|Default|GetSpringArm) (Math|Rotator|CombineRotators (Transformation|GetWorldRotation (Variables|Default|GetSpringArm)) (Math|Rotator|MakeRotator 0.0 0.0 (* AxisValue -4.0))) false false)))

(event Input|MouseEvents|LeftMouseButton
  (params (Key :type Key%20Structure))
  (:Pressed
    (Variables|Default|SetShouldRotated true))
  (:Released
    (Variables|Default|SetShouldRotated false)))

(event Input|MouseEvents|RightMouseButton
  (params (Key :type Key%20Structure))
  (:Pressed
    (Transformation|SetRelativeLocationAndRotation (Variables|Default|GetSpringArm) "0.000000,0.000000,120.000000" "5.000000,-180.000000,0.000000" false false)
    (Variables|/Script/Engine.SpringArmComponent|SetTargetArmLength (Variables|Default|GetSpringArm) 1.6e+02)))

(event Input|MouseEvents|MouseWheelUp
  (params (Key :type Key%20Structure))
  (:Pressed
    (Variables|/Script/Engine.SpringArmComponent|SetTargetArmLength (Variables|Default|GetSpringArm) (Math|Float|Clamp(Float) (- (Variables|/Script/Engine.SpringArmComponent|GetTargetArmLength (Variables|Default|GetSpringArm)) 2e+01) 1e+02 1.8e+02))))

(event Input|MouseEvents|MouseWheelDown
  (params (Key :type Key%20Structure))
  (:Pressed
    (Variables|/Script/Engine.SpringArmComponent|SetTargetArmLength (Variables|Default|GetSpringArm) (Math|Float|Clamp(Float) (+ (Variables|/Script/Engine.SpringArmComponent|GetTargetArmLength (Variables|Default|GetSpringArm)) 2e+01) 1e+02 1.8e+02))))

(fn ConstructionScript)

(fn CreatePlayerDisplay
  (bind _returnvalue (UserInterface|CreateWidget "/Game/Inventory_System/UI/WB_PlayerDisplay.WB_PlayerDisplay_C"))
  (bind _output_get (Variables|Default|SetPlayerDisplay _returnvalue))
  (UserInterface|Viewport|AddtoViewport _output_get 0))

(fn OpenInventory
  (bind _returnvalue (Game|GetPlayerController 0))
  (Rendering|SceneCapture|ShowOnlyActorComponents (Variables|Default|GetSceneCaptureComponent2D) (Variables|Default|GetWardrobe) false)
  (CallFunction|CreatePlayerDisplay)
  (Input|DisableInput (CallFunction|GetHero) _returnvalue)
  (Input|EnableInput _returnvalue))

(fn CloseInventory
  (bind _returnvalue (Game|GetPlayerController 0))
  (bind _playerdisplay (Variables|Default|GetPlayerDisplay)
    (:then
      (Widget|RemovefromParent _playerdisplay)
      (Variables|Default|SetWardrobe 0)
      (Input|DisableInput _returnvalue)
      (Input|EnableInput (CallFunction|GetHero) _returnvalue)
      (Actor|DestroyActor))
    (:else)))

(fn CreateContainerDisplay
  (params (ContainerInventory :type BPC%20Inventory%20Object%20Reference))
  (bind _returnvalue (UserInterface|CreateWidget "/Game/Inventory_System/UI/WB_ContainerDisplay.WB_ContainerDisplay_C" 0 ContainerInventory))
  (bind _output_get (Variables|Default|SetContainerDisplay _returnvalue))
  (UserInterface|Viewport|AddtoViewport _output_get 0))

(fn OpenContainer
  (params (ContainrInventory :type BPC%20Inventory%20Object%20Reference))
  (bind _returnvalue (Game|GetPlayerController 0))
  (Rendering|SceneCapture|ShowOnlyActorComponents (Variables|Default|GetSceneCaptureComponent2D) (Variables|Default|GetWardrobe) false)
  (CallFunction|CreateContainerDisplay ContainrInventory)
  (Input|DisableInput (CallFunction|GetHero) _returnvalue)
  (Input|EnableInput _returnvalue)
  (return (Variables|Default|GetContainerDisplay)))

(fn CloseContainer
  (bind _returnvalue (Game|GetPlayerController 0))
  (bind _containerdisplay (Variables|Default|GetContainerDisplay)
    (:then
      (Widget|RemovefromParent _containerdisplay)
      (Variables|Default|SetWardrobe 0)
      (Input|EnableInput (CallFunction|GetHero) _returnvalue)
      (Input|DisableInput _returnvalue)
      (Actor|DestroyActor))
    (:else)))