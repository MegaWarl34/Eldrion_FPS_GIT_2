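; BP_itemBase is the base actor for inventory items that supplies a "Pick up" prompt with the item's name when looked at.
; Its construction script disables mesh physics and applies the static mesh and materials from the data table row referenced by the BPCItemData component.
; On destruction it adds itself to the game mode's SGBLevelData removed-actor list, without duplicates.
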(event EventBeginPlay)

(event Collision|EventActorBeginOverlap
  (params (OtherActor :type Actor%20Object%20Reference)))

(event EventTick
  (params (DeltaSeconds :type Float%20%28single-precision%29)))

(event EventDestroyed
  (bind _asbp_third_person_game_mode (Utilities|Casting|CastToBP_ThirdPersonGameMode (Game|GetGameMode)))
  (Utilities|Array|AddUnique (Variables|/Game/SaveSystem/SGB_LevelData.SGB_LevelData_C|GetActorRemoved (Variables|/Game/ThirdPerson/Blueprints/BP_ThirdPersonGameMode.BP_ThirdPersonGameMode_C|GetSGB_LevelData _asbp_third_person_game_mode)) (Utilities|ResolveSoftReference self)))

(fn ConstructionScript
  (Physics|SetSimulatePhysics (Variables|Default|GetItemMesh) false)
  (CallFunction|SetItemMesh)
  (CallFunction|SetItemMaterial))

(fn GetItemData
  (bind _bpc_itemdata (Variables|Default|GetBPC_ItemData))
  (bind _itemdata (Variables|/Game/Inventory_System/ItemData/BPC_ItemData.BPC_ItemData_C|GetItemData _bpc_itemdata))
  (bind _returnvalue (Utilities|GetDataTableRow (.datatable _itemdata) (.rowname _itemdata))
    (:then
      (return _returnvalue))))

(fn SetItemMesh
  (Components|StaticMesh|SetStaticMesh (Variables|Default|GetItemMesh) (Utilities|Struct|BreakS_ItemMeshInfo (Utilities|Struct|BreakS_ItemInfo (CallFunction|GetItemData)))))

(fn SetItemMaterial
  (for (_array_element _array_index) (.Material (Utilities|Struct|BreakS_ItemMeshInfo (Utilities|Struct|BreakS_ItemInfo (CallFunction|GetItemData))))
    (Rendering|Material|SetMaterial (Variables|Default|GetItemMesh) _array_index _array_element)))

(fn Lookat
  (return (Utilities|Text|FormatText "Pick up {Item}" (Utilities|Struct|BreakS_ItemInfo (CallFunction|GetItemData)))))