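; Inventory item inspection actor that shows a selected item's 3D mesh for the player to rotate and zoom.
; BeginInspect restricts a SceneCapture2D to its own components, applies mesh and materials from DT_ItemData, enables input and opens WB_InspectItemUI.
; Left-drag rotates the mesh, the wheel zooms via clamped spring arm length, and middle click resets the view.
; Right click or IA_Inventory calls EndInspect, which disables input, removes the widget and destroys the actor.
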(event Input|EnhancedActionEvents|EnhancedInputActionIA_Inventory
  (params (ActionValue :type Boolean) (ElapsedSeconds :type Float%20%28double-precision%29) (TriggeredSeconds :type Float%20%28double-precision%29) (InputAction :type Input%20Action%20Object%20Reference :default "/Game/ThirdPerson/Input/Actions/IA_Inventory.IA_Inventory"))
  (:Started
    (CallFunction|EndInspect)))

(event EventBeginPlay)

(event Collision|EventActorBeginOverlap
  (params (OtherActor :type Actor%20Object%20Reference)))

(event EventTick
  (params (DeltaSeconds :type Float%20%28single-precision%29)))

(event Input|MouseEvents|MouseX
  (params (AxisValue :type Float%20%28single-precision%29))
  (if (Variables|Default|GetShouldRotate)
    (Transformation|SetWorldRotation (Variables|Default|GetInspectMesh) (Math|Rotator|CombineRotators (Transformation|GetWorldRotation (Variables|Default|GetInspectMesh)) (Math|Rotator|MakeRotator 0.0 0.0 (* AxisValue -4.0))) false false)))

(event Input|MouseEvents|MouseY
  (params (AxisValue :type Float%20%28single-precision%29))
  (if (Variables|Default|GetShouldRotate)
    (Transformation|SetWorldRotation (Variables|Default|GetInspectMesh) (Math|Rotator|CombineRotators (Transformation|GetWorldRotation (Variables|Default|GetInspectMesh)) (Math|Rotator|MakeRotator 0.0 (* AxisValue -4.0) 0.0)) false false)))

(event Input|MouseEvents|LeftMouseButton
  (params (Key :type Key%20Structure :default "None"))
  (:Pressed
    (Variables|Default|SetShouldRotate true))
  (:Released
    (Variables|Default|SetShouldRotate false)))

(event Input|MouseEvents|MiddleMouseButton
  (params (Key :type Key%20Structure :default "None"))
  (:Pressed
    (Variables|/Script/Engine.SpringArmComponent|SetTargetArmLength (Variables|Default|GetSpringArm) 1.4e+02)
    (Transformation|SetRelativeLocationAndRotation (Variables|Default|GetInspectMesh) "0, 0, 0" "0, 0, 0" false false)))

(event Input|MouseEvents|MouseWheelDown
  (params (Key :type Key%20Structure :default "None"))
  (:Pressed
    (Variables|/Script/Engine.SpringArmComponent|SetTargetArmLength (Variables|Default|GetSpringArm) (Math|Float|Clamp(Float) (+ (Variables|/Script/Engine.SpringArmComponent|GetTargetArmLength (Variables|Default|GetSpringArm)) 2e+01) 1e+02 2e+02))))

(event Input|MouseEvents|MouseWheelUp
  (params (Key :type Key%20Structure :default "None"))
  (:Pressed
    (Variables|/Script/Engine.SpringArmComponent|SetTargetArmLength (Variables|Default|GetSpringArm) (Math|Float|Clamp(Float) (- (Variables|/Script/Engine.SpringArmComponent|GetTargetArmLength (Variables|Default|GetSpringArm)) 2e+01) 1e+02 2e+02))))

(event Input|MouseEvents|RightMouseButton
  (params (Key :type Key%20Structure :default "None"))
  (:Pressed
    (CallFunction|EndInspect)))

(fn ConstructionScript)

(fn CreateItemInspect
  (bind _returnvalue (UserInterface|CreateWidget "/Game/Inventory_System/Inspect/UI/WB_InspectItemUI.WB_InspectItemUI_C" 0 (Variables|Default|GetInventory) (Variables|Default|GetIndex)))
  (bind _output_get (Variables|Default|SetInspect%20Item _returnvalue))
  (UserInterface|Viewport|AddtoViewport _output_get 0))

(fn GetItemMesh
  (bind _returnvalue (Utilities|GetDataTableRow "/Game/Inventory_System/ItemData/DT_ItemData.DT_ItemData" (Utilities|Struct|BreakS_ItemSlots (Utilities|Array|Get(acopy) (Variables|/Game/Inventory_System/BPC_Inventory.BPC_Inventory_C|GetItemSlots (Variables|Default|GetInventory)) (Variables|Default|GetIndex))))
    (:then
      (return (Utilities|Struct|BreakS_ItemInfo _returnvalue)))))

(fn BeginInspect
  (bind _mesh (CallFunction|GetItemMesh))
  (bind (_staticmesh _material) (Utilities|Struct|BreakS_ItemMeshInfo _mesh))
  (Rendering|SceneCapture|ShowOnlyActorComponents (Variables|Default|GetSceneCaptureComponent2D) self false)
  (Components|StaticMesh|SetStaticMesh (Variables|Default|GetInspectMesh) _staticmesh)
  (for (_array_element _array_index) _material
    (Rendering|Material|SetMaterial (Variables|Default|GetInspectMesh) _array_index _array_element)
    (Input|EnableInput (Game|GetPlayerController 0))
    (CallFunction|CreateItemInspect)))

(fn EndInspect
  (Input|DisableInput (Game|GetPlayerController 0))
  (bind _inspect_item (Variables|Default|GetInspect%20Item)
    (:then
      (Widget|RemovefromParent _inspect_item)
      (Variables|Default|SetInspect%20Item 0)
      (Actor|DestroyActor))
    (:else)))