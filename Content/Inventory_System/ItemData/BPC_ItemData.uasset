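; Item data component that makes its owning actor a pickup, holding an item row and quantity.
; On interaction it requires the interactor's hotbar component, trying it first only when the inventory has no matching slot.
; Matching items or failed hotbar pickups go to the inventory component instead.
; The owner is destroyed after hotbar success or any inventory attempt, whose result goes unchecked; LookAt returns empty text.
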(event Custom|PickUpItem
  (params (Interactor :type Actor%20Object%20Reference))
  (bind _returnvalue (Actor|GetComponentbyClass Interactor "/Game/Inventory_System/BPC_Inventory.BPC_Inventory_C"))
  (bind _returnvalue_2 (Actor|GetComponentbyClass Interactor "/Game/Inventory_System/BPC_Hotbar.BPC_Hotbar_C"))
  (Utilities|IsValid _returnvalue_2
    (:Is%20Valid
      (bind _notsucces (CallFunction|CheckInventory Interactor))
      (if _notsucces
        (bind _sucess (Default|PickUp _returnvalue_2 (.RowName (Utilities|Struct|BreakDataTableRowHandle (Variables|Default|GetItemData))) (Variables|Default|GetItemQuantity)))
        (if _sucess
          (Actor|DestroyActor (Components|GetOwner))
          (else
            (Utilities|IsValid _returnvalue :!label _label
              (:Is%20Valid
                (Default|PickUp _returnvalue (.RowName (Utilities|Struct|BreakDataTableRowHandle (Variables|Default|GetItemData))) (Variables|Default|GetItemQuantity))
                (if true
                  (Actor|DestroyActor (Components|GetOwner)))))))
        (else
          (goto _label))))))

(event EventBeginPlay)

(event EventTick
  (params (DeltaSeconds :type Float%20%28single-precision%29)))

(event EventInteractwith
  (params (Interactor :type Actor%20Object%20Reference))
  (CallFunction|PickUpItem Interactor))

(fn CheckInventory
  (params (Target :type Actor%20Object%20Reference))
  (bind _returnvalue (Actor|GetComponentbyClass Target "/Game/Inventory_System/BPC_Inventory.BPC_Inventory_C"))
  (Utilities|IsValid _returnvalue
    (:Is%20Valid
      (bind _sucess (Default|FindMatchingSlots _returnvalue (.RowName (Utilities|Struct|BreakDataTableRowHandle (Variables|Default|GetItemData)))))
      (return (not _sucess)))))

(fn Lookat
  (return ""))