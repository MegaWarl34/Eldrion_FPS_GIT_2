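; Weather system actor that runs a looping 24-hour day/night cycle with changing weather, scaled by a configurable day length.
; Tick advances the clock, pitches Sun and Moon oppositely from a curve, then calls UpdateWeather; the construction script also applies this in the editor.
; UpdateWeather samples time-of-day curves, blending lighting, atmosphere and fog color between clear and cloudy, driving volumetric cloud material parameters and toggling player-attached rain, snow, lightning and star effects.
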(event Custom|RecaptureSky)

(event EventBeginPlay
  (bind _returnvalue (Game|Player|GetPlayerPawn 0))
  (bind _rootcomponent (Variables|/Script/Engine.Actor|GetRootComponent _returnvalue))
  ;[1 1 1] Event day
  (Variables|Default|SetOneHour (/ (* (Variables|Default|GetDayLenghtMinute) 6e+01) 24.0))
  (Transformation|AttachComponentToComponent (Variables|Default|GetRainComponent) _rootcomponent "None" "SnapToTarget" "KeepRelative" "KeepRelative" true)
  (Transformation|AttachComponentToComponent (Variables|Default|GetSnowComponent) _rootcomponent "None" "SnapToTarget" "KeepRelative" "KeepRelative" true)
  (Transformation|AttachComponentToComponent (Variables|Default|GetStarsComponents) (Variables|/Script/Engine.Actor|GetRootComponent (Game|GetPlayerCharacter 0)) "None" "KeepRelative" "KeepRelative" "KeepRelative" true)
  (Transformation|AttachComponentToComponent (Variables|Default|GetLightningComponent) (Variables|/Script/Engine.Actor|GetRootComponent (Game|GetPlayerCharacter 0)) "None" "KeepRelative" "KeepRelative" "KeepRelative" true))

(event EventTick
  (params (DeltaSeconds :type Float%20%28single-precision%29))
  ;[1 1 1] Event calcul day
  (if (> (+ (Math|Float|SafeDivide DeltaSeconds (Variables|Default|GetOneHour)) (Variables|Default|GetCurrentTime)) 0.0)
    (if (<= (+ (Math|Float|SafeDivide DeltaSeconds (Variables|Default|GetOneHour)) (Variables|Default|GetCurrentTime)) 24.0)
      (Variables|Default|SetCurrentTime (+ (Math|Float|SafeDivide DeltaSeconds (Variables|Default|GetOneHour)) (Variables|Default|GetCurrentTime)))
      (else
        (Variables|Default|SetCurrentTime (Math|Float|Absolute(Float) (- 24.0 (+ (Math|Float|SafeDivide DeltaSeconds (Variables|Default|GetOneHour)) (Variables|Default|GetCurrentTime)))))))
    (Transformation|SetActorRotation (Variables|Default|GetSun) (Math|Rotator|MakeRotator 0.0 (Math|Curves|GetFloatValue (Variables|Default|GetDayLenghtCurve) (Variables|Default|GetCurrentTime)) 0.0))
    (Transformation|SetActorRotation (Variables|Default|GetMoon) (Math|Rotator|MakeRotator 0.0 (* (Math|Curves|GetFloatValue (Variables|Default|GetDayLenghtCurve) (Variables|Default|GetCurrentTime)) -1.0) 0.0))
    (CallFunction|UpdateWeather)))

(fn ConstructionScript
  (Transformation|SetActorLocation (Math|Conversions|ToVector(Float) (Class|GameplayStatics|GetWorldOriginLocation)) false false)
  (Utilities|IsValid (Variables|Default|GetSun)
    (:Is%20Valid
      (Utilities|IsValid (Variables|Default|GetMoon)
        (:Is%20Valid
          (Utilities|IsValid (Variables|Default|GetSkyLight)
            (:Is%20Valid
              (Utilities|IsValid (Variables|Default|GetSkyAtmosphere)
                (:Is%20Valid
                  (Utilities|IsValid (Variables|Default|GetVolumetric%20Cloud)
                    (:Is%20Valid
                      (Utilities|IsValid (Variables|Default|GetFog)
                        (:Is%20Valid
                          (Transformation|SetActorRotation (Variables|Default|GetSun) (Math|Rotator|MakeRotator 0.0 (Math|Curves|GetFloatValue (Variables|Default|GetDayLenghtCurve) (Variables|Default|GetCurrentTime)) 0.0))
                          (Transformation|SetActorRotation (Variables|Default|GetMoon) (Math|Rotator|MakeRotator 0.0 (* (Math|Curves|GetFloatValue (Variables|Default|GetDayLenghtCurve) (Variables|Default|GetCurrentTime)) -1.0) 0.0))
                          (bind _returnvalue (Rendering|Material|CreateDynamicMaterialInstance "/Game/DinCloudsTutorialContent/MIchaelKinseys_CloudsDemo/Materials/MI_Volumetric_Clouds_v2.MI_Volumetric_Clouds_v2" "None" "None" :!class /Script/Engine.KismetMaterialLibrary))
                          (bind _output_get (Variables|Default|SetMID_VolumetricCloud _returnvalue))
                          (Rendering|Material|SetMaterial (Variables|/Script/Engine.VolumetricCloud|GetVolumetricCloudComponent (Variables|Default|GetVolumetric%20Cloud)) _output_get)
                          (CallFunction|UpdateWeather))))))))))))))

(fn UpdateWeather
  (bind _currenttime (Variables|Default|GetCurrentTime))
  (bind _sunintensitycurve (Variables|Default|GetSunIntensityCurve))
  (bind _skylightintensitycurve (Variables|Default|GetSkyLightIntensityCurve))
  (bind _currenttime_2 (Variables|Default|GetCurrentTime))
  (bind _sun (Variables|Default|GetSun))
  (bind _currenttime_3 (Variables|Default|GetCurrentTime))
  (bind _moonintensitycurve (Variables|Default|GetMoonIntensityCurve))
  (bind _rayleightdistributioncurve (Variables|Default|GetRayleightDistributionCurve))
  (bind _currenttime_4 (Variables|Default|GetCurrentTime))
  (bind _currenttime_5 (Variables|Default|GetCurrentTime))
  (bind _daylenghtminute (Variables|Default|GetDayLenghtMinute))
  (bind _starsrotationspeed (Variables|Default|GetStarsRotationSpeed))
  (bind _returnvalue (Math|Curves|GetVectorValue _skylightintensitycurve _currenttime_2))
  (bind _returnvalue_2 (Actor|GetComponentbyClass _sun "/Script/Engine.DirectionalLightComponent"))
  (bind _returnvalue_3 (Math|Curves|GetVectorValue _rayleightdistributioncurve _currenttime_4))
  (bind _returnvalue_4 (Math|Curves|GetVectorValue _moonintensitycurve _currenttime_5))
  (bind _returnvalue_5 (Math|Curves|GetVectorValue _sunintensitycurve _currenttime))
  (bind (_x _y) (Math|Vector|BreakVector _starsrotationspeed))
  (LocalVariables|SetWeatherType (Math|Curves|GetFloatValue (Variables|Default|GetWeatherTypeCurve) (Variables|Default|GetCurrentTime)))
  (Rendering|Components|Light|SetIntensity (Variables|/Script/Engine.Light|GetLightComponent (Variables|Default|GetSun)) (Math|Float|Lerp (.x _returnvalue_5) (.y _returnvalue_5) (LocalVariables|GetWeatherType)))
  (Rendering|Components|Light|SetIntensity (Variables|/Script/Engine.Light|GetLightComponent (Variables|Default|GetMoon)) (Math|Float|Lerp (.x _returnvalue_4) (.y _returnvalue_4) (LocalVariables|GetWeatherType)))
  (Rendering|Components|Light|SetIntensity (Variables|/Script/Engine.SkyLight|GetLightComponent (Variables|Default|GetSkyLight)) (Math|Float|Lerp (.x _returnvalue) (.y _returnvalue) (LocalVariables|GetWeatherType)))
  (if (> (.y (Math|Curves|GetVectorValue (Variables|Default|GetCloudOpacityCurve) (Variables|Default|GetCurrentTime))) 0.5)
    (Components|Activation|Activate (Variables|Default|GetLightningComponent) false)
    (else
      (Components|Activation|Deactivate (Variables|Default|GetLightningComponent))))
  (if (Variables|Default|GetbRain)
    (if (Math|Float|NearlyEqual(Float) (Math|Curves|GetFloatValue (Variables|Default|GetRainTimelineCurve) (Variables|Default|GetCurrentTime)) 1.0 1e-06)
      (Components|Activation|Activate (Variables|Default|GetRainComponent) false)
      (else
        (Components|Activation|Deactivate (Variables|Default|GetRainComponent))))
    (else
      (Components|Activation|Deactivate (Variables|Default|GetRainComponent))))
  (if (Variables|Default|GetbSnow)
    (if (Math|Float|NearlyEqual(Float) (Math|Curves|GetFloatValue (Variables|Default|GetSnowTimelineCurve) (Variables|Default|GetCurrentTime)) 1.0 1e-06)
      (Components|Activation|Activate (Variables|Default|GetSnowComponent) false)
      (else
        (Components|Activation|Deactivate (Variables|Default|GetSnowComponent))))
    (else
      (Components|Activation|Deactivate (Variables|Default|GetSnowComponent))))
  (if (Variables|Default|GetbFog)
    (Class|ExponentialHeightFogComponent|SetFogDensity (Variables|/Script/Engine.ExponentialHeightFog|GetComponent (Variables|Default|GetFog)) (Math|Curves|GetFloatValue (Variables|Default|GetFogTimelineCurve) (Variables|Default|GetCurrentTime)))
    (Class|ExponentialHeightFogComponent|SetFogHeightFalloff (Variables|/Script/Engine.ExponentialHeightFog|GetComponent (Variables|Default|GetFog)) (Math|Curves|GetFloatValue (Variables|Default|GetFogHeightFalloffCurve) (Variables|Default|GetCurrentTime)))
    (else
      (Class|ExponentialHeightFogComponent|SetFogDensity (Variables|/Script/Engine.ExponentialHeightFog|GetComponent (Variables|Default|GetFog)) 0.001)
      (Class|ExponentialHeightFogComponent|SetFogHeightFalloff (Variables|/Script/Engine.ExponentialHeightFog|GetComponent (Variables|Default|GetFog)) 0.2)))
  (if (and (> _currenttime_3 6.0) (< _currenttime_3 18.0))
    (Class|LightComponent|SetEnableLightShaftBloom _returnvalue_2 true)
    (Class|DirectionalLightComponent|SetEnableLightShaftOcclusion _returnvalue_2 true)
    (else
      (Class|LightComponent|SetEnableLightShaftBloom _returnvalue_2 false)
      (Class|DirectionalLightComponent|SetEnableLightShaftOcclusion _returnvalue_2 false)))
  (Class|SkyAtmosphereComponent|SetRayleighExponentialDistribution (Variables|/Script/Engine.SkyAtmosphere|GetSkyAtmosphereComponent (Variables|Default|GetSkyAtmosphere)) (Math|Float|Lerp (.x _returnvalue_3) (.y _returnvalue_3) (LocalVariables|GetWeatherType)))
  (Class|SkyAtmosphereComponent|SetRayleighScattering (Variables|/Script/Engine.SkyAtmosphere|GetSkyAtmosphereComponent (Variables|Default|GetSkyAtmosphere)) (Math|Color|Lerp(LinearColor) (Variables|Default|GetSunnySkyColor) (Variables|Default|GetCloudySkyColor) (LocalVariables|GetWeatherType)))
  (Class|ExponentialHeightFogComponent|SetFogInscatteringColor (Variables|/Script/Engine.ExponentialHeightFog|GetComponent (Variables|Default|GetFog)) (Math|Color|Lerp(LinearColor) (Class|CurveLinearColor|GetClampedLinearColorValue (Variables|Default|GetFogSunnyColor) (Math|Float|NormalizetoRange (Variables|Default|GetCurrentTime) 0.0 24.0)) (Class|CurveLinearColor|GetClampedLinearColorValue (Variables|Default|GetFog%20Cloudy%20Color) (Math|Float|NormalizetoRange (Variables|Default|GetCurrentTime) 0.0 24.0)) (Math|Curves|GetFloatValue (Variables|Default|GetWeatherTypeCurve) (Variables|Default|GetCurrentTime))))
  (Rendering|Material|SetScalarParameterValue (Variables|Default|GetMID_VolumetricCloud) "StratusCoverage" (.x (Math|Curves|GetVectorValue (Variables|Default|GetCloudOpacityCurve) (Variables|Default|GetCurrentTime))) :!class /Script/Engine.MaterialInstanceDynamic)
  (Rendering|Material|SetScalarParameterValue (Variables|Default|GetMID_VolumetricCloud) "CumulonimbusCoverage" (.y (Math|Curves|GetVectorValue (Variables|Default|GetCloudOpacityCurve) (Variables|Default|GetCurrentTime))) :!class /Script/Engine.MaterialInstanceDynamic)
  (Rendering|Material|SetScalarParameterValue (Variables|Default|GetMID_VolumetricCloud) "CloudSpeedX" (Math|Float|SafeDivide (Variables|Default|GetCloudSpeedX) (Variables|Default|GetDayLenghtMinute)) :!class /Script/Engine.MaterialInstanceDynamic)
  (Rendering|Material|SetScalarParameterValue (Variables|Default|GetMID_VolumetricCloud) "CloudSpeedY" (Math|Float|SafeDivide (Variables|Default|GetCloudSpeedY) (Variables|Default|GetDayLenghtMinute)) :!class /Script/Engine.MaterialInstanceDynamic)
  (if (Math|Float|NearlyEqual(Float) (Math|Curves|GetFloatValue (Variables|Default|GetStarscurve) (Variables|Default|GetCurrentTime)) 0.0 1e-06)
    (Components|Activation|Activate (Variables|Default|GetStarsComponents) false)
    (Niagara|SetNiagaraVariable(Vector3) (Variables|Default|GetStarsComponents) "StardomRotation" (Math|Vector|MakeVector (/ _x _daylenghtminute) (/ _y _daylenghtminute) 0.0))
    (else
      (Components|Activation|Deactivate (Variables|Default|GetStarsComponents)))))